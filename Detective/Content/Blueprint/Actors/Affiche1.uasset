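; Affiche1 is an interactable poster actor that opens its UI_Affiche1 widget when the player uses the Intéragir action nearby.
; A Box overlap volume enables the actor's input for player controller 0 on entry and disables it on exit.
; On interaction it sets EnDiscussion on the GI game instance, adds the widget to the viewport and shows the mouse cursor.
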(event `self.Box.OnComponentBeginOverlap`
  (params (OverlappedComponent :type "PrimitiveComponent Object Reference") (OtherActor :type "Actor Object Reference") (OtherComp :type "PrimitiveComponent Object Reference") (OtherBodyIndex :type Integer) (bFromSweep :type Boolean) (SweepResult :type "HitResult Structure (by ref)"))
  ;[1 1 1] Enable/Disable Input
  (`self.EnableInput` (`GameplayStatics.GetPlayerController` 0)))

(event `self.Box.OnComponentEndOverlap`
  (params (OverlappedComponent :type "PrimitiveComponent Object Reference") (OtherActor :type "Actor Object Reference") (OtherComp :type "PrimitiveComponent Object Reference") (OtherBodyIndex :type Integer))
  ;[1 1 1] Enable/Disable Input
  (`self.DisableInput` (`GameplayStatics.GetPlayerController` 0)))

(event `InputAction|Intéragir`
  (params (Key :type "Key Structure"))
  (bind _returnvalue (`GameplayStatics.GetPlayerController` 0))
  (:`Pressed`
    ;[1 1 1] Crée et Affiche UI_Affiche1
    (bind _asgi (cast `/Game/Blueprint/GI` (`GameplayStatics.GetGameInstance`)))
    (set `/Game/Blueprint/GI.EnDiscussion` true _asgi)
    (bind _returnvalue_2 (`|CreateWidget` "/Game/Blueprint/UIs/Affiches/UI_Affiche1.UI_Affiche1_C" _returnvalue))
    (`UserWidget.AddToViewport` _returnvalue_2 0)
    (set `PlayerController.bShowMouseCursor` true _returnvalue)))

(fn `UserConstructionScript`)