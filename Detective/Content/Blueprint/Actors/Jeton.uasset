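; Jeton is a collectible token actor that the player picks up with the Intéragir input action.
; Its Box overlap enables input on entry and disables it on exit, gating the interaction by proximity.
; Pickup destroys the actor and sets PossedeJeton in the GI game instance.
; On BeginPlay it destroys itself if that flag is already true, so a collected token does not reappear.
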(event `self.Box.OnComponentBeginOverlap`
  (params (OverlappedComponent :type "PrimitiveComponent Object Reference") (OtherActor :type "Actor Object Reference") (OtherComp :type "PrimitiveComponent Object Reference") (OtherBodyIndex :type Integer) (bFromSweep :type Boolean) (SweepResult :type "HitResult Structure (by ref)"))
  ;[1 1 1] Enable/Disable Input
  (`self.EnableInput` (`GameplayStatics.GetPlayerController` 0)))

(event `self.Box.OnComponentEndOverlap`
  (params (OverlappedComponent :type "PrimitiveComponent Object Reference") (OtherActor :type "Actor Object Reference") (OtherComp :type "PrimitiveComponent Object Reference") (OtherBodyIndex :type Integer))
  ;[1 1 1] Enable/Disable Input
  (`self.DisableInput` (`GameplayStatics.GetPlayerController` 0)))

(event `InputAction|Intéragir`
  (params (Key :type "Key Structure"))
  (:`Pressed`
    ;[1 1 1] Supprime le Jeton
    (`self.K2_DestroyActor`)
    ;[1 1 1] Posséde le Jeton : True
    (bind _asgi (cast `/Game/Blueprint/GI` (`GameplayStatics.GetGameInstance`)))
    (set `/Game/Blueprint/GI.PossedeJeton` true _asgi)))

(event `self.ReceiveBeginPlay`
  ;[1 1 1] Quand le Jeton est créé, si le joueur posséde deja le Jeton, l'objet est surppimé
  (bind _asgi (cast `/Game/Blueprint/GI` (`GameplayStatics.GetGameInstance`)))
  (if (`/Game/Blueprint/GI.PossedeJeton` _asgi)
    (`self.K2_DestroyActor`)))

(fn `UserConstructionScript`)