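; Interactive door actor that opens and closes when the player presses the Intéragir input, provided the game instance says they own the token (PossedeJeton).
; A Box overlap enables and disables the actor's input for player controller 0.
; DoorClosed toggles a timeline forward or in reverse to drive the mesh's world yaw.
; A DoOnce on the timeline's update sets AOuvertPorte in the game instance the first time the door moves.
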(event `self.Box.OnComponentBeginOverlap`
  (params (OverlappedComponent :type "PrimitiveComponent Object Reference") (OtherActor :type "Actor Object Reference") (OtherComp :type "PrimitiveComponent Object Reference") (OtherBodyIndex :type Integer) (bFromSweep :type Boolean) (SweepResult :type "HitResult Structure (by ref)"))
  ;[1 1 1] Enable/Disable Input
  (`self.EnableInput` (`GameplayStatics.GetPlayerController` 0)))

(event `self.Box.OnComponentEndOverlap`
  (params (OverlappedComponent :type "PrimitiveComponent Object Reference") (OtherActor :type "Actor Object Reference") (OtherComp :type "PrimitiveComponent Object Reference") (OtherBodyIndex :type Integer))
  ;[1 1 1] Enable/Disable Input
  (`self.DisableInput` (`GameplayStatics.GetPlayerController` 0)))

(event `InputAction|Intéragir`
  (params (Key :type "Key Structure"))
  (:`Pressed`
    ;[1 1 1] Vérifie que le Joueur posséde le Jeton
    (bind _asgi (cast `/Game/Blueprint/GI` (`GameplayStatics.GetGameInstance`)))
    (if (`/Game/Blueprint/GI.PossedeJeton` _asgi)
      ;[1 1 1] Open/Close Door
      (if (`self.Door Closed`)
        (set `self.Door Closed` false)
        (bind (_direction _open_close_door) (`Timeline|Open/Close Door` :!label _label)
          (:`Update`
            (`SceneComponent.K2_SetWorldRotation` (`self.StaticMesh`) (`KismetMathLibrary.MakeRotator` 0.0 0.0 _open_close_door) false false)
            (`/Engine/EditorBlueprintResources/StandardMacros.DoOnce` false
              (:`Completed`
                (set `/Game/Blueprint/GI.AOuvertPorte` true _asgi)))))
        (else
          (set `self.Door Closed` true)
          (goto _label :!via `Reverse`))))))

(fn `UserConstructionScript`)