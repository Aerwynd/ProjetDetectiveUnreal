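; Game Instance that handles saving, loading and deleting the player's progress in a single save slot.
; On Init it loads the existing Objets_Sauvegarder save object or creates a new one, without applying it.
; Save and load functions copy player location, notoriety, an NPC dialogue flag and token possession between the game and a PlayerLevelData struct.
; Delete removes the slot but leaves the in-memory save object untouched.
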(event `self.ReceiveInit`
  (bind _returnvalue (`GameplayStatics.DoesSaveGameExist` "SaveSlotName"))
  (if _returnvalue
    (bind _returnvalue_2 (`GameplayStatics.LoadGameFromSlot` "SaveSlotName"))
    (bind _asobjets_sauvegarder (cast `/Game/Blueprint/Sauvegarde/Objets_Sauvegarder` _returnvalue_2))
    (set `self.Save Game Data` _asobjets_sauvegarder)
    (else
      (bind _returnvalue_3 (`GameplayStatics.CreateSaveGameObject` "/Game/Blueprint/Sauvegarde/Objets_Sauvegarder.Objets_Sauvegarder_C"))
      (set `self.Save Game Data` _returnvalue_3))))

(fn `Delete Data `
  (`GameplayStatics.DeleteGameInSlot` "SaveSlotName"))

(fn `Load Data Player`
  (locals (PlayerRef :type "/Game/Blueprint/ThirdPersonCharacter Object Reference"))
  (bind (_player_level_data_location `_player_level_data_notoriété` `_player_level_data_aparléaconducteurtrain` _player_level_data_possedejeton) (break `/Game/Blueprint/Sauvegarde/PlayerSaveData` (`/Game/Blueprint/Sauvegarde/Objets_Sauvegarder.Player/Level Data` (`self.Save Game Data`))))
  (bind _asthird_person_character (cast `/Game/Blueprint/ThirdPersonCharacter` (`GameplayStatics.GetPlayerCharacter` 0)))
  (bind _output_get (set `local.PlayerRef` _asthird_person_character))
  (`Actor.K2_SetActorLocation` _output_get _player_level_data_location false false)
  (set `self.NotoriétéActuelle` `_player_level_data_notoriété`)
  (set `self.AParléAvecPNJ1` `_player_level_data_aparléaconducteurtrain`)
  (set `self.PossedeJeton` _player_level_data_possedejeton))

(fn `SaveData Player`
  (locals (`Player Ref` :type "/Game/Blueprint/ThirdPersonCharacter Object Reference"))
  (bind _save_game_data (`self.Save Game Data`))
  (bind _asthird_person_character (cast `/Game/Blueprint/ThirdPersonCharacter` (`GameplayStatics.GetPlayerCharacter` 0)))
  (bind _output_get (set `local.Player Ref` _asthird_person_character))
  (set `/Game/Blueprint/Sauvegarde/Objets_Sauvegarder.Player/Level Data` (make `/Game/Blueprint/Sauvegarde/PlayerSaveData` (`Actor.K2_GetActorLocation` _output_get) (`self.NotoriétéActuelle`) (`self.AParléAvecPNJ1`) (`self.PossedeJeton`)) _save_game_data)
  (bind _returnvalue (`GameplayStatics.SaveGameToSlot` _save_game_data "SaveSlotName"))
  (`KismetSystemLibrary.PrintString` (`KismetStringLibrary.Conv_BoolToString` _returnvalue)))