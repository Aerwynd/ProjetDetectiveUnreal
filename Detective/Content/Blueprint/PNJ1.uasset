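; PNJ1 is an NPC actor that opens its UI_PNJ1 widget when F is pressed within its trigger box.
; Box overlap events toggle the prompt text and enable or disable the actor's input.
; Pressing F clears the GI game instance's EnDiscussion flag, adds a new widget to the viewport and hides the cursor.
; Ending overlap removes that widget and also hides the cursor.
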(event `self.Box.OnComponentBeginOverlap`
  (params (OverlappedComponent :type "PrimitiveComponent Object Reference") (OtherActor :type "Actor Object Reference") (OtherComp :type "PrimitiveComponent Object Reference") (OtherBodyIndex :type Integer) (bFromSweep :type Boolean) (SweepResult :type "HitResult Structure (by ref)"))
  (`self.EnableInput` (`GameplayStatics.GetPlayerController` 0))
  (`SceneComponent.ToggleVisibility` (`self.TextRender`) false))

(event `self.Box.OnComponentEndOverlap`
  (params (OverlappedComponent :type "PrimitiveComponent Object Reference") (OtherActor :type "Actor Object Reference") (OtherComp :type "PrimitiveComponent Object Reference") (OtherBodyIndex :type Integer))
  (bind _returnvalue (`GameplayStatics.GetPlayerController` 0))
  (`self.DisableInput` _returnvalue)
  (`SceneComponent.ToggleVisibility` (`self.TextRender`) false)
  (set `PlayerController.bShowMouseCursor` false _returnvalue)
  (`Widget.RemoveFromParent` (stale `Key|F` _returnvalue_2)))

(event `Key|F`
  (params (Key :type "Key Structure"))
  (bind _returnvalue (`GameplayStatics.GetPlayerController` 0))
  (:`Pressed`
    (bind _asgi (cast `/Game/Blueprint/GI` (`GameplayStatics.GetGameInstance`)))
    (set `/Game/Blueprint/GI.EnDiscussion` false _asgi)
    (bind _returnvalue_2 (`|CreateWidget` "/Game/Blueprint/UI_PNJ1.UI_PNJ1_C" _returnvalue))
    (`UserWidget.AddToViewport` _returnvalue_2 0)
    (set `PlayerController.bShowMouseCursor` false _returnvalue)))

(fn `UserConstructionScript`)