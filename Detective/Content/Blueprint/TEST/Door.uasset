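; Door actor that the player toggles with the E key, available only while holding a token (PossédeJeton in the GI game instance).
; Box1 overlap enables input and toggles the TextRender's visibility if the token is owned; leaving disables input and toggles it again.
; E flips DoorOpen and plays or reverses the OpenDoor timeline, which drives the door's world yaw.
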(event `self.Box1.OnComponentBeginOverlap`
  (params (OverlappedComponent :type "PrimitiveComponent Object Reference") (OtherActor :type "Actor Object Reference") (OtherComp :type "PrimitiveComponent Object Reference") (OtherBodyIndex :type Integer) (bFromSweep :type Boolean) (SweepResult :type "HitResult Structure (by ref)"))
  (bind _returnvalue (`GameplayStatics.GetPlayerController` 0))
  (bind _asgi (cast `/Game/Blueprint/GI` (`GameplayStatics.GetGameInstance`)))
  (if (`/Game/Blueprint/GI.PossédeJeton` _asgi)
    (`self.EnableInput` _returnvalue)
    (`SceneComponent.ToggleVisibility` (`self.TextRender`) false)
    (else
      (`self.DisableInput` _returnvalue))))

(event `self.Box1.OnComponentEndOverlap`
  (params (OverlappedComponent :type "PrimitiveComponent Object Reference") (OtherActor :type "Actor Object Reference") (OtherComp :type "PrimitiveComponent Object Reference") (OtherBodyIndex :type Integer))
  (`self.DisableInput` (`GameplayStatics.GetPlayerController` 0))
  (`SceneComponent.ToggleVisibility` (`self.TextRender`) false))

(event `Key|E`
  (params (Key :type "Key Structure"))
  (:`Pressed`
    (if (`self.DoorOpen`)
      (set `self.DoorOpen` false)
      (bind (_direction _open_close_door) (`Timeline|openDoor` :!label _label)
        (:`Update`
          (`SceneComponent.K2_SetWorldRotation` (`self.door`) (`KismetMathLibrary.MakeRotator` 0.0 0.0 _open_close_door) false false)))
      (else
        (set `self.DoorOpen` true)
        (goto _label :!via `Reverse`)))))

(fn `UserConstructionScript`)